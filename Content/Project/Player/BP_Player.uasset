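; BP_Player is the player character, with a state enum (Default, Splint, Guard, Observe) gating movement, dodge and speed.
; Splint, a sprint, orients the body to movement, Guard changes walk speed, and Dodge either jumps or plays a rolling montage by state.
; Observe frees the camera from body yaw; on release, Tick interpolates control yaw back to actor yaw, restoring Default once within tolerance.
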(event `self.ReceiveTick`
  (params (DeltaSeconds :type "Float (single-precision)"))
  (switch `/Game/Project/Player/BluePrints/E_PlayerState` (`self.ECurrentState`)
    (:`NewEnumerator1`
      (`self.ResetObserve` DeltaSeconds))))

(event `/Game/Project/Interfaces/BI_Move.MoveX`
  (params (InputX :type "Float (double-precision)") (ControllerYawRotator :type "Rotator Structure"))
  (bind (_inputdirection_x _inputdirection_y _inputdirection_z) (`KismetMathLibrary.BreakVector` (`self.InputDirection`)))
  (set `self.InputDirection` (`KismetMathLibrary.MakeVector` InputX _inputdirection_y _inputdirection_z))
  (switch `/Game/Project/Player/BluePrints/E_PlayerState` (`self.ECurrentState`)
    (:`NewEnumerator0`
      _)
    (:`NewEnumerator2`
      _)
    (:`NewEnumerator3`
      _))
  (`self.AddMovementInput` (`KismetMathLibrary.GetForwardVector` ControllerYawRotator) InputX))

(event `/Game/Project/Interfaces/BI_Dodge.Dodge`
  ; Dodge
  (switch `/Game/Project/Player/BluePrints/E_PlayerState` (`self.ECurrentState`)
    (:`NewEnumerator0`
      (`self.Jump` :!label _label))
    (:`NewEnumerator1`
      (goto _label))
    (:`NewEnumerator2`
      (if true :!label _label_2
        (`|PlayMontage` (`self.Mesh`) "/Game/Project/Player/Animations/MT_Rolling.MT_Rolling")))
    (:`NewEnumerator3`
      (goto _label_2))))

(event `/Game/Project/Interfaces/BI_Move.MoveY`
  (params (InputY :type "Float (double-precision)") (ControllerYawRotator :type "Rotator Structure"))
  (bind (_inputdirection_x _inputdirection_y _inputdirection_z) (`KismetMathLibrary.BreakVector` (`self.InputDirection`)))
  (set `self.InputDirection` (`KismetMathLibrary.MakeVector` _inputdirection_x InputY _inputdirection_z))
  (switch `/Game/Project/Player/BluePrints/E_PlayerState` (`self.ECurrentState`)
    (:`NewEnumerator0`
      _)
    (:`NewEnumerator2`
      _)
    (:`NewEnumerator3`
      _))
  (`self.AddMovementInput` (`KismetMathLibrary.GetRightVector` ControllerYawRotator) InputY))

(event `/Game/Project/Interfaces/BI_Look.RotateYaw`
  (params (InputX :type "Float (double-precision)"))
  (`self.AddControllerYawInput` InputX))

(event `/Game/Project/Interfaces/BI_Splint.Splint`
  (bind _charactermovement (`self.CharacterMovement`))
  ; Splint
  (switch `/Game/Project/Player/BluePrints/E_PlayerState` (`self.ECurrentState`)
    (:`NewEnumerator0`
      (set `self.ECurrentState` "NewEnumerator2")
      (set `CharacterMovementComponent.MaxWalkSpeed` (`self.SplintSpeed`) _charactermovement)
      (set `self.bUseControllerRotationYaw` false)
      (set `CharacterMovementComponent.bOrientRotationToMovement` true _charactermovement))))

(event `/Game/Project/Interfaces/BI_Look.RotatePitch`
  (params (InputY :type "Float (double-precision)"))
  (`self.AddControllerPitchInput` InputY))

(event `/Game/Project/Interfaces/BI_Splint.StopSplint`
  (bind _charactermovement (`self.CharacterMovement`))
  ; Splint
  (switch `/Game/Project/Player/BluePrints/E_PlayerState` (`self.ECurrentState`)
    (:`NewEnumerator2`
      (set `self.ECurrentState` "NewEnumerator0")
      (set `CharacterMovementComponent.MaxWalkSpeed` (`self.BaseSpeed`) _charactermovement)
      (set `self.bUseControllerRotationYaw` true)
      (set `CharacterMovementComponent.bOrientRotationToMovement` false _charactermovement))))

(event `/Game/Project/Interfaces/BI_Observe.Observe`
  (switch `/Game/Project/Player/BluePrints/E_PlayerState` (`self.ECurrentState`)
    (:`NewEnumerator0`
      (set `self.ECurrentState` "NewEnumerator1")
      (set `self.bUseControllerRotationYaw` false)
      (set `self.IsFixedForward` false))))

(event `/Game/Project/Interfaces/BI_Guard.Guard`
  ; 가드
  (switch `/Game/Project/Player/BluePrints/E_PlayerState` (`self.ECurrentState`)
    (:`NewEnumerator0`
      (set `self.ECurrentState` "NewEnumerator3")
      (set `CharacterMovementComponent.MaxWalkSpeed` (`self.GuardSpeed`) (`self.CharacterMovement`)))))

(event `/Game/Project/Interfaces/BI_Observe.StopObserve`
  (switch `/Game/Project/Player/BluePrints/E_PlayerState` (`self.ECurrentState`)
    (:`NewEnumerator1`
      (set `self.IsFixedForward` true))))

(event `/Game/Project/Interfaces/BI_Guard.StopGuard`
  ; 가드
  (switch `/Game/Project/Player/BluePrints/E_PlayerState` (`self.ECurrentState`)
    (:`NewEnumerator3`
      (set `self.ECurrentState` "NewEnumerator0")
      (set `CharacterMovementComponent.MaxWalkSpeed` (`self.BaseSpeed`) (`self.CharacterMovement`)))))

(event `/Game/Project/Interfaces/BI_Observe.ResetObserve`
  (params (DeltaTime :type "Float (double-precision)"))
  (if (and (`self.IsFixedForward`) (== (`self.ECurrentState`) (`KismetMathLibrary.Conv_ByteToInt` (enumliteral `/Game/Project/Player/BluePrints/E_PlayerState` "NewEnumerator1"))))
    (bind (_controlleryaw _actoryaw) (`self.InterpYaw` DeltaTime))
    (`self.IsCloserThanTorelance` _controlleryaw _actoryaw 10.0
      (:`True`
        (set `self.bUseControllerRotationYaw` true)
        (set `self.IsFixedForward` false)
        (set `self.ECurrentState` "NewEnumerator0")))))

(fn `InterpYaw`
  (params (DeltaTime :type "Float (double-precision)"))
  (returns (ControllerYaw :type "Float (double-precision)") (ActorYaw :type "Float (double-precision)"))
  (bind _returnvalue (`self.GetControlRotation`))
  (bind _yaw (.yaw (`self.K2_GetActorRotation`)))
  (`Controller.SetControlRotation` (`self.GetController`) (`KismetMathLibrary.RInterpTo` _returnvalue (`KismetMathLibrary.MakeRotator` (.roll _returnvalue) (.pitch _returnvalue) _yaw) DeltaTime (`self.CameraRotateSpeed`)))
  (return (.yaw _returnvalue) _yaw))

(fn `UserConstructionScript`)
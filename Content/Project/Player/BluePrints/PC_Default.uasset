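; Default player controller that turns Enhanced Input actions into commands for the player character.
; On BeginPlay it adds the default mapping context and caches the player pawn, cast to BP_Player, as the playable character.
; Dodge, attack, sprint, guard and observe actions forward as message calls, with start and stop pairs for held inputs.
; Move passes axes with a yaw-only control rotation, while look forwards yaw and pitch separately.
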(event `self.ReceiveBeginPlay`
  (`EnhancedInputSubsystemInterface.AddMappingContext` (pcsubsystem `EnhancedInputLocalPlayerSubsystem` self) "/Game/Project/Inputs/IMC_Default.IMC_Default" 0 (struct))
  (bind _asbp_player (cast `/Game/Project/Player/BP_Player` (`GameplayStatics.GetPlayerPawn` 0)))
  (set `self.PlayableCharacter` _asbp_player))

(event `EnhancedInput|/Game/Project/Inputs/IA_Dodge`
  (params (ActionValue :type Boolean) (ElapsedSeconds :type "Float (double-precision)") (TriggeredSeconds :type "Float (double-precision)") (InputAction :type "InputAction Object Reference" :default "/Game/Project/Inputs/IA_Dodge.IA_Dodge"))
  (:`Started`
    (message `/Game/Project/Interfaces/BI_Dodge.Dodge` (`self.PlayableCharacter`))))

(event `EnhancedInput|/Game/Project/Inputs/IA_Attack1`
  (params (ActionValue :type Boolean) (ElapsedSeconds :type "Float (double-precision)") (TriggeredSeconds :type "Float (double-precision)") (InputAction :type "InputAction Object Reference" :default "/Game/Project/Inputs/IA_Attack1.IA_Attack1"))
  (:`Started`
    (`/Game/Project/Player/BP_Player.Attack1` (`self.PlayableCharacter`))))

(event `EnhancedInput|/Game/Project/Inputs/IA_Move`
  (params (ActionValue :type "Vector2D Structure") (ElapsedSeconds :type "Float (double-precision)") (TriggeredSeconds :type "Float (double-precision)") (InputAction :type "InputAction Object Reference" :default "/Game/Project/Inputs/IA_Move.IA_Move"))
  (bind (_returnvalue_roll _returnvalue_pitch _returnvalue_yaw) (`KismetMathLibrary.BreakRotator` (`self.GetControlRotation`)))
  (bind _playablecharacter (`self.PlayableCharacter`))
  (bind _returnvalue (`KismetMathLibrary.MakeRotator` 0.0 0.0 _returnvalue_yaw))
  (:`Triggered`
    (message `/Game/Project/Interfaces/BI_Move.MoveX` _playablecharacter ActionValue_Y _returnvalue)
    (message `/Game/Project/Interfaces/BI_Move.MoveY` _playablecharacter ActionValue_X _returnvalue)))

(event `EnhancedInput|/Game/Project/Inputs/IA_Splint`
  (params (ActionValue :type Boolean) (ElapsedSeconds :type "Float (double-precision)") (TriggeredSeconds :type "Float (double-precision)") (InputAction :type "InputAction Object Reference" :default "/Game/Project/Inputs/IA_Splint.IA_Splint"))
  (bind _playablecharacter (`self.PlayableCharacter`))
  (:`Triggered`
    (message `/Game/Project/Interfaces/BI_Splint.Splint` _playablecharacter))
  (:`Completed`
    (message `/Game/Project/Interfaces/BI_Splint.StopSplint` _playablecharacter)))

(event `EnhancedInput|/Game/Project/Inputs/IA_Guard`
  (params (ActionValue :type Boolean) (ElapsedSeconds :type "Float (double-precision)") (TriggeredSeconds :type "Float (double-precision)") (InputAction :type "InputAction Object Reference" :default "/Game/Project/Inputs/IA_Guard.IA_Guard"))
  (bind _playablecharacter (`self.PlayableCharacter`))
  (:`Triggered`
    (message `/Game/Project/Interfaces/BI_Guard.Guard` _playablecharacter))
  (:`Completed`
    (message `/Game/Project/Interfaces/BI_Guard.StopGuard` _playablecharacter)))

(event `EnhancedInput|/Game/Project/Inputs/IA_Look`
  (params (ActionValue :type "Vector2D Structure") (ElapsedSeconds :type "Float (double-precision)") (TriggeredSeconds :type "Float (double-precision)") (InputAction :type "InputAction Object Reference" :default "/Game/Project/Inputs/IA_Look.IA_Look"))
  (bind _playablecharacter (`self.PlayableCharacter`))
  (:`Triggered`
    (message `/Game/Project/Interfaces/BI_Look.RotateYaw` _playablecharacter ActionValue_X)
    (message `/Game/Project/Interfaces/BI_Look.RotatePitch` _playablecharacter ActionValue_Y)))

(event `EnhancedInput|/Game/Project/Inputs/IA_Observe`
  (params (ActionValue :type Boolean) (ElapsedSeconds :type "Float (double-precision)") (TriggeredSeconds :type "Float (double-precision)") (InputAction :type "InputAction Object Reference" :default "/Game/Project/Inputs/IA_Observe.IA_Observe"))
  (bind _playablecharacter (`self.PlayableCharacter`))
  (:`Triggered`
    (message `/Game/Project/Interfaces/BI_Observe.Observe` _playablecharacter))
  (:`Completed`
    (message `/Game/Project/Interfaces/BI_Observe.StopObserve` _playablecharacter)))

(fn `UserConstructionScript`)
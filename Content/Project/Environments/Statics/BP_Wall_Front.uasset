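; BP_Wall_Front is an environment wall that opens like a door when the Grux boss dies.
; On BeginPlay it finds the BP_Grux actor in the level and binds OpenDoor to its OnDie event.
; OpenDoor plays a timeline that slides the SmallScene component from its initial location by a scaled OpenAmount offset.
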(event `self.ReceiveBeginPlay`
  (bind _returnvalue (`GameplayStatics.GetActorOfClass` "/Game/Project/NPC/Grux/BP_Grux.BP_Grux_C"))
  (`/Engine/EditorBlueprintResources/StandardMacros.IsValid` _returnvalue
    (:`Is Valid`
      (set `self.BossActor` _returnvalue)
      (add `/Game/Project/NPC/Grux/BP_Grux.OnDie` _returnvalue (delegate `OpenDoor`)))))

(event `OpenDoor`
  (bind (_direction _ratio) (`Timeline|TL_Open`)
    (:`Update`
      (`SceneComponent.K2_SetRelativeLocation` (`self.SmallScene`) (+ (* _ratio (`self.OpenAmount`)) (`self.InitialDoorLocation`)) false false))))

(fn `UserConstructionScript`)
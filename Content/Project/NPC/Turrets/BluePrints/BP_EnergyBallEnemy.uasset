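; BP_EnergyBallEnemy is an energy ball projectile, filed with the NPC turrets, that damages the player on contact.
; FindTargetDirection sets a normalized direction toward a target actor's current location, and Tick moves the ball along it at Speed, scaled by delta time and without sweep.
; On overlap with BP_Player it applies BaseDamage and destroys itself, ignoring all other actors.
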(event `self.ReceiveTick`
  (params (DeltaSeconds :type "Float (single-precision)"))
  (`self.K2_SetActorLocation` (+ (* DeltaSeconds (`self.Speed`) (`self.Direction`)) (`self.K2_GetActorLocation`))))

(event `self.ReceiveActorBeginOverlap`
  (params (OtherActor :type "Actor Object Reference"))
  (bind _asbp_player (cast `/Game/Project/Player/BP_Player` OtherActor))
  (`GameplayStatics.ApplyDamage` _asbp_player (`self.Base Damage`) null self)
  (`self.K2_DestroyActor`))

(event `/Game/Project/Interfaces/BPI_FindTargetDirection.FindTargetDirection`
  (params (TargetActor :type "Actor Object Reference"))
  (set `self.Direction` (`KismetMathLibrary.Normal` (- (`self.K2_GetActorLocation` TargetActor) (`self.K2_GetActorLocation`)))))

(fn `UserConstructionScript`)
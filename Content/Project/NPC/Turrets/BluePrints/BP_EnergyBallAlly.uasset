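; BP_EnergyBallAlly is a projectile, apparently fired by allied turrets, that damages BP_Grux enemies.
; FindTargetDirection stores a normalized direction toward a given target once per call, and Tick moves the ball along it at Speed without sweep or homing.
; On overlapping a BP_Grux it applies BaseDamage and destroys itself, while other overlaps are ignored.
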(event `self.ReceiveTick`
  (params (DeltaSeconds :type "Float (single-precision)"))
  (`self.K2_SetActorLocation` (+ (* DeltaSeconds (`self.Speed`) (`self.Direction`)) (`self.K2_GetActorLocation`))))

(event `self.ReceiveActorBeginOverlap`
  (params (OtherActor :type "Actor Object Reference"))
  (bind _asbp_grux (cast `/Game/Project/NPC/Grux/BP_Grux` OtherActor))
  (`GameplayStatics.ApplyDamage` _asbp_grux (`self.Base Damage`) null self)
  (`self.K2_DestroyActor`))

(event `/Game/Project/Interfaces/BPI_FindTargetDirection.FindTargetDirection`
  (params (TargetActor :type "Actor Object Reference"))
  (set `self.Direction` (`KismetMathLibrary.Normal` (- (`self.K2_GetActorLocation` TargetActor) (`self.K2_GetActorLocation`)))))

(fn `UserConstructionScript`)
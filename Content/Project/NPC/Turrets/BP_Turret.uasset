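; NPC turret that the player wakes and triggers into timed combat while allied, and can damage to death once it turns enemy.
; A Sleep/Wait/Combat/Death state machine gates interaction and attacks through Tick-driven cooldown and combat timers.
; Sphere overlaps pick BP_Grux or the player as target by team, while Attack only toggles a recoil-timed firing flag.
; Timelines animate core brightness and team color on dynamic materials, and turning enemy swaps the cooldown widget for health.
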(event `self.ReceiveBeginPlay`
  (bind _basematerial (`self.BaseMaterial`))
  (bind _coreglow (`self.CoreGlow`))
  ; Begin
  (bind _returnvalue (`PrimitiveComponent.CreateDynamicMaterialInstance` (`self.Mesh`) 2 _basematerial "None"))
  (`KismetArrayLibrary.Array_Add` _coreglow _returnvalue)
  (bind _returnvalue_2 (`PrimitiveComponent.CreateDynamicMaterialInstance` (`self.Mesh`) 6 _basematerial "None"))
  (`KismetArrayLibrary.Array_Add` _coreglow _returnvalue_2)
  (bind _returnvalue_3 (`PrimitiveComponent.CreateDynamicMaterialInstance` (`self.Ring`) 1 _basematerial "None"))
  (`KismetArrayLibrary.Array_Add` _coreglow _returnvalue_3)
  (`WidgetComponent.SetWidget` (`self.Widget`) (`self.CoolTimeWidget`))
  (`SceneComponent.SetVisibility` (`self.Widget`) false false)
  ;; Bind Event to Player Interaction
  (bind _returnvalue_4 (`GameplayStatics.GetActorOfClass` "/Game/Project/Player/BP_Player.BP_Player_C"))
  (add `/Game/Project/Player/BP_Player.AlertInteraction` _returnvalue_4 (delegate `ReceiveInteraction`)))

(event `/Game/Project/Interfaces/BPI_Interaction.Interaction`
  ; Player Interaction: Activate Turrets
  (switch `/Game/Project/NPC/Turrets/BluePrints/E_TurretTeam` (`self.ECurrentTeam`)
    (:`NewEnumerator0`
      (switch `/Game/Project/NPC/Turrets/BluePrints/E_TurretState` (`self.ECurrentState`)
        (:`NewEnumerator0`
          (`self.ChangeToWaitMode`))
        (:`NewEnumerator1`
          (if (<= (`self.CoolTime`) 0.0)
            (`self.ChangeToCombatMode` (`self.CombatDuration`))))))))

(event `ChangeToWaitMode`
  ; Change Mode & Bright : Sleep <> Wait
  (bind (_direction _ratio) (`Timeline|TL_Activate` :!label _label)
    (:`Update`
      (for _array_element (`self.CoreGlow`)
        (`self.ChangeBrightSleepToWait` _array_element _ratio)))
    (:`Finished`
      (switch `ETimelineDirection` _direction
        (:`Forward`
          (set `self.CanAttack` false)
          (set `self.ECurrentState` "NewEnumerator1")
          (`/Game/Project/UI/Widgets/BPI_CoolTime.SetNewCoolTime` 10.0))))))

(event `ChangeToDeath`
  ; Change Mode & Bright : Sleep <> Wait
  (set `self.ECurrentState` "NewEnumerator5")
  (goto _label :!via `Reverse`))

(event `ReceiveInteraction`
  ; Begin
  ;; Bind Event to Player Interaction
  (if (`self.IsPanelOpen`)
    (message `/Game/Project/Interfaces/BPI_Interaction.Interaction` self)))

(event `/Game/Project/UI/Widgets/BPI_CoolTime.SetNewCoolTime`
  (params (CoolTime :type "Float (double-precision)"))
  (bind _cooltimewidget (`self.CoolTimeWidget`))
  ; Set New Cool Time & Update Widgets
  (bind _output_get (set `self.CoolTime` CoolTime))
  (if (`KismetSystemLibrary.DoesImplementInterface` _cooltimewidget "/Game/Project/UI/Widgets/BPI_CoolTime.BPI_CoolTime_C")
    (`/Game/Project/UI/Widgets/BPI_CoolTime.SetNewCoolTime` _cooltimewidget _output_get)))

(event `ChangeToCombatMode`
  (params (CombatDuration :type "Float (double-precision)"))
  ; Change Mode : Wait <> Combat
  (set `self.ECurrentState` "NewEnumerator2")
  (`/Game/Project/UI/Widgets/BPI_CoolTime.SetNewCoolTime` CombatDuration)
  (set `self.RemainCombatTime` CombatDuration)
  (`KismetSystemLibrary.Delay` 3.0)
  (set `self.CanAttack` true))

(event `self.ReceiveTick`
  (params (DeltaSeconds :type "Float (single-precision)"))
  (bind _interactionparticle (`self.InteractionParticle`))
  ; Tick
  (`|ExecutionSequence`
    (:`then_0`
      (`self.DecreaseTimes` DeltaSeconds)
      (if (<= (`self.RemainCombatTime`) 0.0)
        (`self.TurnOffCombatMode`)))
    (:`then_1`
      (if (or (> (`self.CoolTime`) 0.0) (not (`self.IsActivated`)))
        (`ActorComponent.Deactivate` _interactionparticle)
        (else
          (`ActorComponent.Activate` _interactionparticle false))))
    (:`then_2`
      (`self.FindTarget`)
      (if (`self.CanAttack`)
        (`/Engine/EditorBlueprintResources/StandardMacros.IsValid` (`self.TargetActor`)
          (:`Is Valid`
            (if (not (`self.IsFiring`))
              (`self.Attack`))))))))

(event `TurnOffCombatMode`
  ; Change Mode : Wait <> Combat
  (switch `/Game/Project/NPC/Turrets/BluePrints/E_TurretState` (`self.ECurrentState`)
    (:`NewEnumerator2`
      (set `self.CanAttack` false)
      (`self.ChangeToWaitMode`))))

(event `self.ReceiveAnyDamage`
  (params (Damage :type "Float (single-precision)") (DamageType :type "DamageType Object Reference") (InstigatedBy :type "Controller Object Reference") (DamageCauser :type "Actor Object Reference"))
  ; Damaged
  (cast `/Game/Project/Player/BP_Player` DamageCauser)
  (switch `/Game/Project/NPC/Turrets/BluePrints/E_TurretTeam` (`self.ECurrentTeam`)
    (:`NewEnumerator1`
      (bind _isactivated (`self.HitDamage` Damage))
      (if _isactivated
        (`self.PlayAnimMontage` "/Game/Project/NPC/Turrets/Animations/MT_HitReact.MT_HitReact")
        (else
          (`self.ChangeToDeath`)
          (`ActorComponent.Activate` (`self.DieParticle`) false))))))

(event `ChangeToEnemy`
  (bind _healthwidget (`self.HealthWidget`))
  (bind _widget (`self.Widget`))
  ; Change Team & Color : Ally > Enemy
  (`|ExecutionSequence`
    (:`then_0`
      (bind _returnvalue (`self.IsSleep`))
      (if _returnvalue
        (set `self.ECurrentState` "NewEnumerator1")
        (`/Game/Project/UI/Widgets/BPI_CoolTime.SetNewCoolTime` 0.0)))
    (:`then_1`
      (bind (_direction _ratio) (`Timeline|TL_ChangeTeam`)
        (:`Update`
          (for _array_element (`self.CoreGlow`)
            (bind (_element2 _ratio2) (`self.ChangeColorAllyToEnemy` _array_element _ratio))
            (if _returnvalue
              (`self.ChangeBrightSleepToWait` _element2 _ratio2))))
        (:`Finished`
          (set `self.ECurrentTeam` "NewEnumerator1")
          (`WidgetComponent.SetWidget` _widget _healthwidget)
          (`WidgetComponent.SetDrawSize` _widget (200.0 20.0))
          (set `/Game/Project/UI/Widgets/WBP_TurretHealth.HealthPercent` 1.0 _healthwidget)
          (`self.ChangeToCombatMode` 20.0))))))

(event `self.ReceiveActorBeginOverlap`
  (params (OtherActor :type "Actor Object Reference"))
  ; Overlap
  (cast `/Game/Project/Player/BP_Player` OtherActor)
  (set `self.IsPanelOpen` true)
  (`SceneComponent.SetVisibility` (`self.Widget`) (`self.IsActivated`) false))

(event `self.ReceiveActorEndOverlap`
  (params (OtherActor :type "Actor Object Reference"))
  ; Overlap
  (cast `/Game/Project/Player/BP_Player` OtherActor)
  (set `self.IsPanelOpen` false)
  (`SceneComponent.SetVisibility` (`self.Widget`) false false))

(event `Attack`
  ; Attack
  (set `self.IsFiring` true)
  (`KismetSystemLibrary.Delay` (`self.RecoilDuration`))
  (set `self.IsFiring` false))

(fn `DecreaseTimes`
  (params (DeltaTime :type "Float (double-precision)"))
  (`|ExecutionSequence`
    (:`then_0`
      (bind _output_get (set `self.CoolTime` (`KismetMathLibrary.FClamp` (- (`self.CoolTime`) DeltaTime) 0.0 (`self.CoolTime`))))
      (set `/Game/Project/UI/Widgets/WBP_TurretCoolTime.CoolTime` _output_get (`self.CoolTimeWidget`)))
    (:`then_1`
      (set `self.RemainCombatTime` (`KismetMathLibrary.FClamp` (- (`self.RemainCombatTime`) DeltaTime) 0.0 (`self.RemainCombatTime`))))))

(fn `FindTarget`
  (bind _returnvalue (`self.K2_GetActorLocation`))
  (bind _array (`|MakeArray` "ObjectTypeQuery3" :!type "EObjectTypeQuery Enum"))
  (bind _attackrange (`self.AttackRange`))
  (switch `/Game/Project/NPC/Turrets/BluePrints/E_TurretState` (`self.ECurrentState`)
    (:`NewEnumerator1`
      _)
    (:`NewEnumerator2`
      _))
  (switch `/Game/Project/NPC/Turrets/BluePrints/E_TurretTeam` (`self.ECurrentTeam`)
    (:`NewEnumerator0`
      (bind (_outactors _returnvalue_2) (`KismetSystemLibrary.SphereOverlapActors` _returnvalue _attackrange _array "/Game/Project/NPC/Grux/BP_Grux.BP_Grux_C"))
      (set `self.TargetActor` (`|GetArrayItem` _outactors))
      (set `self.IsAiming` _returnvalue_2))
    (:`NewEnumerator1`
      (bind (_outactors_2 _returnvalue_3) (`KismetSystemLibrary.SphereOverlapActors` _returnvalue _attackrange _array "/Game/Project/Player/BP_Player.BP_Player_C"))
      (set `self.TargetActor` (`|GetArrayItem` _outactors_2))
      (set `self.IsAiming` _returnvalue_3))))

(fn `HitDamage`
  (params (Damage :type "Float (double-precision)"))
  (returns (IsActivated :type Boolean))
  (bind _output_get (set `self.CurrentHealth` (`KismetMathLibrary.FClamp` (- (`self.CurrentHealth`) Damage) 0.0 (`self.MaxHealth`))))
  (set `/Game/Project/UI/Widgets/WBP_TurretHealth.HealthPercent` (/ _output_get (`self.MaxHealth`)) (`self.HealthWidget`))
  (bind _output_get_2 (set `self.IsActivated` (> _output_get 0.0)))
  (return _output_get_2))

(fn `IsSleep`
  (returns (ReturnValue :type Boolean))
  (return (== (`self.ECurrentState`) (`KismetMathLibrary.Conv_ByteToInt` (enumliteral `/Game/Project/NPC/Turrets/BluePrints/E_TurretState` "NewEnumerator0")))))

(fn `UserConstructionScript`)
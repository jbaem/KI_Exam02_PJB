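; Grux enemy NPC with montage-driven sword, rush, slide and stamp attacks.
; Begin/End trace events set flags that Tick turns into once-per-window capsule-trace damage, while Stamp converts nearby turrets to enemies.
; Right and big swings also trace the left sword, leaving RightSwordTracing unused.
; Damage updates health and AIC_Grux, then either signals death or targets the attacker in the blackboard, playing directional hit reacts past a damage threshold.
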(event `self.ReceiveTick`
  (params (DeltaSeconds :type "Float (single-precision)"))
  (`self.DamageTracing`))

(event `self.ReceiveAnyDamage`
  (params (Damage :type "Float (single-precision)") (DamageType :type "DamageType Object Reference") (InstigatedBy :type "Controller Object Reference") (DamageCauser :type "Actor Object Reference"))
  (`self.LostHealth` Damage)
  (bind _asaic_grux (cast `/Game/Project/NPC/Grux/BluePrints/AIC_Grux` (`AIBlueprintHelperLibrary.GetAIController` self)))
  (`/Game/Project/NPC/Grux/BluePrints/AIC_Grux.OnReceiveDamage` _asaic_grux (/ (`self.CurrentHealth`) (`self.MaxHealth`)))
  (`self.OnDamaged`)
  (if (> (`self.CurrentHealth`) 0.0)
    (`self.PlayHitReactMontage` DamageCauser)
    (`BlackboardComponent.SetValueAsObject` (`AIBlueprintHelperLibrary.GetBlackboard` (`self.GetController`)) (`self.PlayerActorKey`) DamageCauser)
    (else
      (set `self.IsDead` true)
      (`self.OnDie`))))

(event `self.Rush`
  (bind _charactermovement (`self.CharacterMovement`))
  (set `self.MoveSpeedCached` (`CharacterMovementComponent.MaxWalkSpeed` _charactermovement))
  (set `CharacterMovementComponent.MaxWalkSpeed` 800.0 _charactermovement)
  (`|AIMoveTo` (`AIBlueprintHelperLibrary.GetAIController` self) null (0.0 0.0 0.0) (`GameplayStatics.GetPlayerPawn` 0)
    (:`OnSuccess`
      _)
    (:`OnFail`
      _))
  (`|PlayMontage` (`self.Mesh`) "/Game/Project/NPC/Grux/Animations/MT_RushAttack.MT_RushAttack"
    (:`OnCompleted`
      _)
    (:`OnInterrupted`
      _))
  (set `CharacterMovementComponent.MaxWalkSpeed` (`self.MoveSpeedCached`) (`self.CharacterMovement`)))

(event `self.Attack1`
  (`|PlayMontage` (`self.Mesh`) "/Game/Project/NPC/Grux/Animations/MT_Attack1.MT_Attack1"))

(event `self.Attack3`
  (`|PlayMontage` (`self.Mesh`) "/Game/Project/NPC/Grux/Animations/MT_BigAttack.MT_BigAttack"))

(event `self.BeginTraceStamp`
  (set `self.IsStampTracing` true)
  (`KismetArrayLibrary.Array_Clear` (`self.AlreadyHitActor`)))

(event `self.EndTraceStamp`
  (set `self.IsStampTracing` false))

(event `self.BeginTraceBig`
  (set `self.IsBigTracing` true)
  (`KismetArrayLibrary.Array_Clear` (`self.AlreadyHitActor`)))

(event `self.EndTraceBig`
  (set `self.IsBigTracing` false))

(event `self.Attack2`
  (`|PlayMontage` (`self.Mesh`) "/Game/Project/NPC/Grux/Animations/MT_Attack2.MT_Attack2"))

(event `self.Attack4`
  (`|PlayMontage` (`self.Mesh`) "/Game/Project/NPC/Grux/Animations/MT_SlideAttack.MT_SlideAttack"))

(event `self.BeginTraceRush`
  (set `self.IsRushTracing` true)
  (`KismetArrayLibrary.Array_Clear` (`self.AlreadyHitActor`)))

(event `self.EndTraceRush`
  (set `self.IsRushTracing` false))

(event `self.BeginTraceRight`
  (set `self.IsRightTracing` true)
  (`KismetArrayLibrary.Array_Clear` (`self.AlreadyHitActor`)))

(event `self.EndTraceRight`
  (set `self.IsRightTracing` false))

(event `self.Stamp`
  (`|PlayMontage` (`self.Mesh`) "/Game/Project/NPC/Grux/Animations/MT_Stamp.MT_Stamp"))

(event `self.BeginTraceLeft`
  (set `self.IsLeftTracing` true)
  (`KismetArrayLibrary.Array_Clear` (`self.AlreadyHitActor`)))

(event `self.EndTraceLeft`
  (set `self.IsLeftTracing` false))

(fn `Attack`
  (returns (Duration :type "Float (double-precision)"))
  (bind _returnvalue (`self.PlayAnimMontage` "/Game/Project/NPC/Grux/Animations/MT_BigAttack.MT_BigAttack"))
  (return _returnvalue))

(fn `GetHitDirection`
  (params (Causer :type "Actor Object Reference"))
  (returns (ReturnValue_X :type "Float (double-precision)") (ReturnValue_Y :type "Float (double-precision)"))
  (bind (_returnvalue_x _returnvalue_y) (`KismetMathLibrary.BreakVector` (`KismetMathLibrary.InverseTransformDirection` (`self.GetTransform`) (`KismetMathLibrary.Normal` (- (`self.K2_GetActorLocation` Causer) (`self.K2_GetActorLocation`))))))
  (return _returnvalue_x _returnvalue_y))

(fn `GetRandomLocation`
  (returns (Location :type "Vector Structure"))
  (bind _randomlocation (`NavigationSystemV1.K2_GetRandomLocationInNavigableRadius` (`self.K2_GetActorLocation`) (`self.RandomMoveRadius`) null null))
  (return _randomlocation))

(fn `UserConstructionScript`)
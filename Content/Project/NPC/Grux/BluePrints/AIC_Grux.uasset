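; AI controller for the Grux NPC that runs its behavior tree and drives a health-based, multi-phase fight through Blackboard keys.
; Perception updates containing the player store it as the target and change the state, with no path that clears sight.
; Damage events update health and advance the combat phase one step at a time by threshold, flagging each change.
; Zero health sets a final state.
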(event `self.ReceiveBeginPlay`
  (bind _returnvalue (`AIBlueprintHelperLibrary.GetBlackboard` null))
  (`self.RunBehaviorTree` "/Game/Project/NPC/Grux/BluePrints/BT_Grux.BT_Grux")
  (`BlackboardComponent.SetValueAsEnum` _returnvalue "EState" 0)
  (`BlackboardComponent.SetValueAsInt` _returnvalue "CombatPhase" 1)
  (`BlackboardComponent.SetValueAsFloat` _returnvalue "CurrentHealthPercent" 100.0))

(event `self.AIPerception.OnPerceptionUpdated`
  (params (UpdatedActors :type "Array of Actor Object Reference (by ref)"))
  (bind _returnvalue (`AIBlueprintHelperLibrary.GetBlackboard` null))
  (for _array_element UpdatedActors
    (bind _asbp_player (cast `/Game/Project/Player/BP_Player` _array_element))
    (`BlackboardComponent.SetValueAsBool` _returnvalue "CanSeePlayer" true)
    (`BlackboardComponent.SetValueAsObject` _returnvalue "PlayerActor" _asbp_player)
    (`BlackboardComponent.SetValueAsEnum` _returnvalue "EState" 1)))

(event `OnReceiveDamage`
  (params (CurrentHealthPercent :type "Float (double-precision)"))
  (bind _returnvalue (`AIBlueprintHelperLibrary.GetBlackboard` null))
  (bind _returnvalue_2 (`AIBlueprintHelperLibrary.GetBlackboard` null))
  (bind _returnvalue_3 (`AIBlueprintHelperLibrary.GetBlackboard` null))
  (`BlackboardComponent.SetValueAsFloat` (`AIBlueprintHelperLibrary.GetBlackboard` null) "CurrentHealthPercent" CurrentHealthPercent)
  (if (> CurrentHealthPercent 0.7)
    (if (== (`self.CurrentPhase`) 0)
      (bind _output_get (set `self.CurrentPhase` 1))
      (`BlackboardComponent.SetValueAsInt` _returnvalue (`self.CombatPhase`) _output_get)
      (`BlackboardComponent.SetValueAsBool` _returnvalue "IsChangedPhase" true)
      (`BlackboardComponent.SetValueAsEnum` _returnvalue "EState" 2))
    (elif (> CurrentHealthPercent 0.3)
      (if (== (`self.CurrentPhase`) 1)
        (bind _output_get_2 (set `self.CurrentPhase` 2))
        (`BlackboardComponent.SetValueAsInt` _returnvalue_2 (`self.CombatPhase`) _output_get_2)
        (`BlackboardComponent.SetValueAsBool` _returnvalue_2 "IsChangedPhase" true))
      (elif (> CurrentHealthPercent 0.0)
        (if (== (`self.CurrentPhase`) 2)
          (bind _output_get_3 (set `self.CurrentPhase` 3))
          (`BlackboardComponent.SetValueAsInt` _returnvalue_3 (`self.CombatPhase`) _output_get_3)
          (`BlackboardComponent.SetValueAsBool` _returnvalue_3 "IsChangedPhase" true))
        (else
          (`BlackboardComponent.SetValueAsEnum` (`AIBlueprintHelperLibrary.GetBlackboard` null) "EState" 3))))))

(fn `UserConstructionScript`)
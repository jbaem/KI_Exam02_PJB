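; Anim notify state for Grux's left attack that marks the window during which the left-side attack trace runs.
; On notify begin and end, it checks that the mesh owner implements BPI_GruxAttackTracing, then sends BeginTraceLeftMessage or EndTraceLeftMessage.
; The tracing itself is left to the owning actor, reached only through the interface.
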(fn `Received_NotifyBegin`
  (params (MeshComp :type "SkeletalMeshComponent Object Reference") (Animation :type "AnimSequenceBase Object Reference") (TotalDuration :type "Float (single-precision)") (EventReference :type "AnimNotifyEventReference Structure (by ref)"))
  (returns (ReturnValue :type Boolean))
  (bind _returnvalue (`ActorComponent.GetOwner` MeshComp))
  (if (`KismetSystemLibrary.DoesImplementInterface` _returnvalue "/Game/Project/NPC/Grux/BluePrints/BPI_GruxAttackTracing.BPI_GruxAttackTracing_C")
    (message `/Game/Project/NPC/Grux/BluePrints/BPI_GruxAttackTracing.BeginTraceLeft` _returnvalue))
  (return false))

(fn `Received_NotifyEnd`
  (params (MeshComp :type "SkeletalMeshComponent Object Reference") (Animation :type "AnimSequenceBase Object Reference") (EventReference :type "AnimNotifyEventReference Structure (by ref)"))
  (returns (ReturnValue :type Boolean))
  (bind _returnvalue (`ActorComponent.GetOwner` MeshComp))
  (if (`KismetSystemLibrary.DoesImplementInterface` _returnvalue "/Game/Project/NPC/Grux/BluePrints/BPI_GruxAttackTracing.BPI_GruxAttackTracing_C")
    (message `/Game/Project/NPC/Grux/BluePrints/BPI_GruxAttackTracing.EndTraceLeft` _returnvalue))
  (return false))
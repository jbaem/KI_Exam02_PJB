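; Grux NPC character that takes damage, reacts to hits and dies, and exposes attack and random navigable-location helpers.
; On damage it clamps health, reports the health ratio to AIC_Grux and fires damaged or death callbacks.
; While alive, it picks one of four directional hit-react montages from the causer's local-space direction.
; Reactions are throttled by accumulated damage, playing only when the sum reaches HitReactDamage, which is then subtracted.
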(event `self.ReceiveAnyDamage`
  (params (Damage :type "Float (single-precision)") (DamageType :type "DamageType Object Reference") (InstigatedBy :type "Controller Object Reference") (DamageCauser :type "Actor Object Reference"))
  (`self.LostHealth` Damage)
  (bind _asaic_grux (cast `/Game/Project/NPC/Grux/BluePrints/AIC_Grux` (`AIBlueprintHelperLibrary.GetAIController` null)))
  (`/Game/Project/NPC/Grux/BluePrints/AIC_Grux.OnReceiveDamage` _asaic_grux (/ (`self.CurrentHealth`) (`self.MaxHealth`)))
  (`self.OnDamaged`)
  (if (> (`self.CurrentHealth`) 0.0)
    (`self.PlaytHitReactMontage` DamageCauser)
    (`KismetSystemLibrary.PrintString` (`KismetStringLibrary.Conv_DoubleToString` (`self.CurrentHealth`)))
    (else
      (set `self.IsDead` true)
      (`self.OnDie`))))

(fn `Attack`
  (returns (Duration :type "Float (double-precision)"))
  (bind _returnvalue (`self.PlayAnimMontage` "/Game/Project/NPC/Grux/Animations/MT_BigAttack.MT_BigAttack"))
  (return _returnvalue))

(fn `GetHitDirection`
  (params (Causer :type "Actor Object Reference"))
  (returns (ReturnValue_X :type "Float (double-precision)") (ReturnValue_Y :type "Float (double-precision)"))
  (bind (_returnvalue_x _returnvalue_y) (`KismetMathLibrary.BreakVector` (`KismetMathLibrary.InverseTransformDirection` (`self.GetTransform`) (`KismetMathLibrary.Normal` (- (`self.K2_GetActorLocation` Causer) (`self.K2_GetActorLocation`))))))
  (return _returnvalue_x _returnvalue_y))

(fn `GetRandomLocation`
  (returns (Location :type "Vector Structure"))
  (bind _randomlocation (`NavigationSystemV1.K2_GetRandomLocationInNavigableRadius` (`self.K2_GetActorLocation`) (`self.RandomMoveRadius`) null null))
  (return _randomlocation))

(fn `UserConstructionScript`)